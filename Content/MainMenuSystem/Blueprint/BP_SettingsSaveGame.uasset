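; Save game data container for the main menu system, holding graphics settings and the player's state.
; Paired setter and getter functions store each quality category (overall graphics, shadows, anti-aliasing, post-processing, view distance, textures, effects) as both a command and an enum target.
; A third pair stores player transform, health and current level.
; The functions only copy variables, with no disk saving or command execution here.
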(fn SettingAllCommands
  (params (Graphics%20Save%20Command :type String) (Shadows%20Save%20Command :type String) (Anti%20Save%20Command :type String) (POST-PROCESSINGSave%20Command :type String) (VIEW%20DISTANCE%20Save%20Command :type String) (TEXTURE%20QUALITY%20Save%20Command :type String) (EFFECTS%20Save%20Command :type String))
  (bind _output_get (Variables|Command|SetGraphics%20Save%20Command Graphics%20Save%20Command))
  (bind _output_get_2 (Variables|Command|SetShadows%20Save%20Command Shadows%20Save%20Command))
  (bind _output_get_3 (Variables|Command|SetAnti%20Save%20Command Anti%20Save%20Command))
  (bind _output_get_4 (Variables|Command|SetPOST-PROCESSINGSave%20Command POST-PROCESSINGSave%20Command))
  (bind _output_get_5 (Variables|Command|SetVIEW%20DISTANCE%20Save%20Command VIEW%20DISTANCE%20Save%20Command))
  (bind _output_get_6 (Variables|Command|SetTEXTURE%20QUALITY%20Save%20Command TEXTURE%20QUALITY%20Save%20Command))
  (bind _output_get_7 (Variables|Command|SetEFFECTS%20Save%20Command EFFECTS%20Save%20Command))
  (return _output_get _output_get_2 _output_get_3 _output_get_4 _output_get_5 _output_get_6 _output_get_7))

(fn SettingAllEnums
  (params (Graphics%20Target :type E_LowToHigh%20Enum :default "NewEnumerator0") (Shadows%20Target :type E_LowToHigh%20Enum :default "NewEnumerator0") (Anti%20Target :type E_LowToHigh%20Enum :default "NewEnumerator0") (POST-PROCESSING%20Target :type E_LowToHigh%20Enum :default "NewEnumerator0") (VIEW%20DISTANCE%20Target :type E_LowToHigh%20Enum :default "NewEnumerator0") (TEXTURE%20QUALITY%20Target :type E_LowToHigh%20Enum :default "NewEnumerator0") (EFFECTS%20Target :type E_LowToHigh%20Enum :default "NewEnumerator0"))
  (Variables|Enums|SetGraphics%20Target Graphics%20Target)
  (Variables|Enums|SetShadows%20Target Shadows%20Target)
  (Variables|Enums|SetAnti%20Target Anti%20Target)
  (Variables|Enums|SetPOST-PROCESSING%20Target POST-PROCESSING%20Target)
  (Variables|Enums|SetVIEW%20DISTANCE%20Target VIEW%20DISTANCE%20Target)
  (Variables|Enums|SetTEXTURE%20QUALITY%20Target TEXTURE%20QUALITY%20Target)
  (Variables|Enums|SetEFFECTS%20Target EFFECTS%20Target))

(fn GettingAllCommands
  (return (Variables|Command|GetGraphics%20Save%20Command) (Variables|Command|GetShadows%20Save%20Command) (Variables|Command|GetAnti%20Save%20Command) (Variables|Command|GetPOST-PROCESSINGSave%20Command) (Variables|Command|GetVIEW%20DISTANCE%20Save%20Command) (Variables|Command|GetTEXTURE%20QUALITY%20Save%20Command) (Variables|Command|GetEFFECTS%20Save%20Command)))

(fn GettingAllEnums
  (return (Variables|Enums|GetGraphics%20Target) (Variables|Enums|GetShadows%20Target) (Variables|Enums|GetAnti%20Target) (Variables|Enums|GetPOST-PROCESSING%20Target) (Variables|Enums|GetVIEW%20DISTANCE%20Target) (Variables|Enums|GetTEXTURE%20QUALITY%20Target) (Variables|Enums|GetEFFECTS%20Target)))

(fn SetPlayerState
  (params (Player%20Location%20And%20Rotations :type Transform) (Player%20Health :type Float%20%28single-precision%29) (Current%20Level :type Name))
  (Variables|Default|SetPlayer%20Location%20And%20Rotations Player%20Location%20And%20Rotations)
  (Variables|Default|SetPlayer%20Health Player%20Health)
  (Variables|Default|SetCurrent%20Level Current%20Level))

(fn GetPlayerState
  (return (Variables|Default|GetPlayer%20Location%20And%20Rotations) (Variables|Default|GetPlayer%20Health) (Variables|Default|GetCurrent%20Level)))